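; Attribute component in the Flashlight folder that tracks a battery energy value.
; ModifyAttribute accepts a gameplay tag and a signed delta, acting only on an exact Attribute.Energy match.
; It clamps the new energy between zero and MaxEnergy, broadcasts OnBatteryChanged with the normalized charge, and prints the raw value.
; BeginPlay is empty, so all changes come through calls to that function.
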(event EventBeginPlay)

(fn ModifyAttribute
  (params (AttributeTag%20 :type Gameplay%20Tag%20Structure) (ModifierValue%20 :type Float%20%28double-precision%29))
  (if (GameplayTags|MatchesTag AttributeTag%20 "(TagName=\"Attribute.Energy\")" true)
    (if (>= ModifierValue%20 0.0)
      (Variables|Default|SetCurrectEnergy (Math|Float|Min(Float) (+ ModifierValue%20 (Variables|Default|GetCurrectEnergy)) (Variables|Default|GetMaxEnergy)))
      (else
        (Variables|Default|SetCurrectEnergy (Math|Float|Max(Float) (+ ModifierValue%20 (Variables|Default|GetCurrectEnergy)) 0.0))))
    (Default|CallOnBatteryChanged (/ (Variables|Default|GetCurrectEnergy) (Variables|Default|GetMaxEnergy)))
    (Development|PrintString (Utilities|String|ToString(Float) (Variables|Default|GetCurrectEnergy)))
    (return)))