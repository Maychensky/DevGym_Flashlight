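; Actor component that removes its owning pickup, with a poof sound, when the pickup is interacted with.
; On BeginPlay it casts the owner to BP_BasePickup and binds to its OnInteracted event, doing nothing if the cast fails.
; On interaction it plays the sound at the owner's location, hides the static mesh, disables the sphere collision and destroys the actor.
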(event Custom|OnOwnerInterected
  (params (Instigator :type Actor%20Object%20Reference))
  (bind _returnvalue (Components|GetOwner))
  (Audio|PlaySoundatLocation "/Game/Flashlight/freesound_community-poof-of-smoke-87381.freesound_community-poof-of-smoke-87381" (Transformation|GetActorLocation _returnvalue) "0, 0, 0" 1.0 1.0 0.0 0 0 0 0)
  (Rendering|SetVisibility (Actor|GetComponentbyClass _returnvalue "/Script/Engine.StaticMeshComponent") false false)
  (Collision|SetCollisionEnabled (Actor|GetComponentbyClass _returnvalue "/Script/Engine.SphereComponent") "NoCollision")
  (Actor|DestroyActor _returnvalue))

(event EventBeginPlay
  (bind _asbp_base_pickup (Utilities|Casting|CastToBP_BasePickup (Components|GetOwner)))
  (EventDispatchers|BindEventtoOnInteracted _asbp_base_pickup (delegate Custom|OnOwnerInterected)))