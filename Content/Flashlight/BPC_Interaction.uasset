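; BPC_Interaction is an interaction component that lets its owner interact with whatever the player camera is looking at.
; TryInteract line-traces on the Visibility channel along the camera's forward vector and sends InteractMessage to hit actors implementing BPI_Interactable, passing the owner.
; On success, it broadcasts the returned item's attribute tag and modifier value through the OnInteractionDataReceived dispatcher, leaving their application to listeners.
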(event EventBeginPlay)

(event EventTick
  (params (DeltaSeconds :type Float%20%28single-precision%29)))

(fn TryInteract
  (bind _returnvalue (Game|GetPlayerCameraManager 0))
  (bind _returnvalue_2 (Camera|GetCameraLocation _returnvalue))
  (bind _outhit (Collision|LineTraceByChannel _returnvalue_2 (+ _returnvalue_2 (* (Transformation|GetActorForwardVector _returnvalue) (Variables|Default|GetLengthTraceLine))) "TraceTypeQuery1" false 0 "None"))
  (if (Utilities|DoesObjectImplementInterface (.HitActor (Collision|BreakHitResult _outhit)) "/Game/Flashlight/BPI_Interactable.BPI_Interactable_C")
    (bind (_itemdata _success) (Class|BPIInteractable|Interact(Message) (.HitActor (Collision|BreakHitResult _outhit)) (Components|GetOwner)))
    (if _success
      (Default|CallOnInteractionDataReceived (.targetattribute _itemdata) (.madifiervalue _itemdata)))))