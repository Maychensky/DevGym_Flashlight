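; BP_ItemSpawner is an actor that spawns an item of a configurable class at its own transform and respawns it after interaction.
; It spawns the first item on BeginPlay, stores it as the current object and binds to its OnInteracted event.
; When that event fires, a short delay leads back into the same spawn logic, which binds the new item and repeats the cycle without destroying the previous one.
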(event Custom|CustomEvent
  (params (Instigator :type Actor%20Object%20Reference))
  (Utilities|FlowControl|Delay 5.0)
  (CallFunction|SpawnLogic))

(event Custom|SpawnLogic
  (bind _returnvalue (Game|SpawnActorfromClass :Class (Variables|Default|GetClass) :SpawnTransform (Transformation|GetActorTransform) :CollisionHandlingOverride "AlwaysSpawn" :TransformScaleMethod "MultiplyWithRoot" :Instigator 0))
  (Variables|Default|SetCurrentSpawnObj _returnvalue)
  (EventDispatchers|BindEventtoOnInteracted (Variables|Default|GetCurrentSpawnObj) (delegate Custom|CustomEvent)))

(event EventBeginPlay
  (CallFunction|SpawnLogic))

(fn ConstructionScript)